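; PC_Player is a player controller that manages the mouse cursor and click interactivity.
; SetCursor maps a cursor-state value to a hardware cursor, using hand shapes for hover and click and hiding it for the directional states.
; LockClick and UnlockClick toggle the IsInteractable flag and reapply Game and UI input mode, with UnlockClick keeping the cursor visible during capture.
; Play begins with clicks unlocked.
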(event EventBeginPlay
  (CallFunction|UnlockClick))

(event EventSetCursor
  (params (Image :type Enum_CursorType%20Enum :default "NewEnumerator0"))
  (Variables|Default|SetCurrentMouseCursor (Utilities|Select :Index Image :NewEnumerator0 "Default" :NewEnumerator1 "None" :NewEnumerator2 "None" :NewEnumerator3 "None" :NewEnumerator4 "None" :NewEnumerator5 "Hand" :NewEnumerator6 "GrabHand")))

(event EventUnlockClick
  (Variables|Default|SetIsInteractable true)
  (Input|SetInputModeGameandUI self 0 "DoNotLock" false false))

(event EventLockClick
  (Variables|Default|SetIsInteractable false)
  (Input|SetInputModeGameandUI self 0 "DoNotLock" true false))

(fn ConstructionScript)