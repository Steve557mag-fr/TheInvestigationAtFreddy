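; Game instance that runs microphone speech recognition for the whole app session and passes recognized text on as voice events.
; On Init it creates and starts a speech recognizer, then opens a capturable sound wave for the microphone.
; Captured audio streams into the recognizer, and each recognized segment fires VoiceDetected.
; Errors print to screen, and Shutdown stops capture and recognition if the capture is valid.
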(event Custom|OnSentenceReceived
  (params (RecognizedWords :type String))
  ;[1 1 1] When the app init
  ;;[0.4301 0.7076 1] When worlds are detected
  (Default|CallVoiceDetected RecognizedWords))

(event Custom|OnStartedSpeechRecognition
  (params (bSucceeded :type Boolean))
  ;[1 1 1] When the app init
  ;;[1 0.6458 0.6458] Start the recognition
  (bind _returnvalue (Class|CapturableSoundWave|CreateCapturableSoundWave))
  (bind _output_get (Variables|Default|SetCurrent%20Capture _returnvalue))
  (EventDispatchers|BindEventtoOnPopulateAudioData _output_get (delegate Custom|OnPopulateAudioData))
  (Class|CapturableSoundWave|StartCapture _output_get))

(event Custom|OnRecogErr
  (params (ShortErrorMessage :type String) (LongErrorMessage :type String))
  ;[1 1 1] When the app init
  ;;[1 0.6354 0.6354] Error when recognition
  (Development|PrintString ShortErrorMessage))

(event Custom|OnPopulateAudioData
  (params (PopulatedAudioData :type Array%20of%20Floats%20%28single-precision%29))
  (bind _current_capture (Variables|Default|GetCurrent%20Capture))
  ;[1 1 1] When the app init
  ;;[0.3665 0.5249 1] Process Audio Data (Proceed to the speech IA)
  (Class|SpeechRecognizer|ProcessAudioData (Variables|Default|GetCurrentSpeechRecognizer) PopulatedAudioData (Math|Conversions|ToFloat(Integer) (Class|ImportedSoundWave|GetSampleRate _current_capture)) (Class|ImportedSoundWave|GetNumOfChannels _current_capture) false))

(event EventInit
  ;[1 1 1] When the app init
  ;;[0.2921 0.6108 1] Create the SVR IAModel
  (bind _returnvalue (Class|SpeechRecognizer|CreateSpeechRecognizer))
  (bind _output_get (Variables|Default|SetCurrentSpeechRecognizer _returnvalue))
  ;;[1 0.6354 0.6354] Error when recognition
  (EventDispatchers|BindEventtoOnRecognitionError _output_get (delegate Custom|OnRecogErr))
  ;;[0.4301 0.7076 1] When worlds are detected
  (EventDispatchers|BindEventtoOnRecognizedTextSegment (Variables|Default|GetCurrentSpeechRecognizer) (delegate Custom|OnSentenceReceived))
  ;;[1 0.6458 0.6458] Start the recognition
  (Class|SpeechRecognizer|StartSpeechRecognition (Variables|Default|GetCurrentSpeechRecognizer) (delegate Custom|OnStartedSpeechRecognition))
  (Development|PrintString "Hello"))

(event EventShutdown
  ;[1 1 1] When the app shutdown
  ;;[0.4316 0.6089 1] Stop the microphone capture + VSR
  (bind _current_capture (Variables|Default|GetCurrent%20Capture)
    (:then
      (Class|CapturableSoundWave|StopCapture _current_capture)
      (Development|PrintString "[VSR]: Disabled")
      (Class|SpeechRecognizer|StopSpeechRecognition (Variables|Default|GetCurrentSpeechRecognizer)))
    (:else)))