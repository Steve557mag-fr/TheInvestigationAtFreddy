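; BP_WorldInteract_Parent is a base Blueprint for clickable world interactions, driven by mouse clicks and cursor hover.
; It caches the PC_Player controller on BeginPlay and, when clicked while that controller is interactable, locks click messages for a Cooldown delay, then unlocks them.
; Hovering sets the player controller's cursor message to an enum state and resets it when the cursor leaves.
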(event EventBeginPlay
  (bind _aspc_player (Utilities|Casting|CastToPC_Player (Game|GetPlayerController 0)))
  (Variables|Default|SetPC_Player _aspc_player))

(event MouseInput|EventActorOnClicked
  (params (ButtonPressed :type Key%20Structure :default "None"))
  (bind _pc_player (Variables|Default|GetPC_Player))
  (if (Variables|/Game/Blueprints/Player/PC_Player.PC_Player_C|GetIsInteractable (Variables|Default|GetPC_Player))
    (Class|BPIInteraction|LockClick(Message) _pc_player)
    (Utilities|FlowControl|Delay (Variables|Default|GetCooldown))
    (Class|BPIInteraction|UnlockClick(Message) _pc_player)))

(event MouseInput|EventActorBeginCursorOver
  (Class|BPIInteraction|SetCursor(Message) (Game|GetPlayerController 0) "NewEnumerator5"))

(event MouseInput|EventActorEndCursorOver
  (Class|BPIInteraction|SetCursor(Message) (Game|GetPlayerController 0) "NewEnumerator0"))

(fn ConstructionScript)